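; BP_Support is a support power actor that drops a bomb, which explodes on impact.
; On BeginPlay it pushes the Bomba component downward with an acceleration-based force scaled by VelocidadCaida, then toggles the cooldown flag in its SpecialAttack struct around a short delay, with debug prints.
; When Bomba hits something, it spawns BP_Explosion at the bomb's transform and destroys itself.
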(event OnComponentHit(Bomba)
  (params (HitComponent :type Primitive%20Component%20Object%20Reference) (OtherActor :type Actor%20Object%20Reference) (OtherComp :type Primitive%20Component%20Object%20Reference) (NormalImpulse :type Vector :default "0, 0, 0") (Hit :type Hit%20Result%20Structure%20%28by%20ref%29))
  (Game|SpawnActorfromClass "/Game/Poderes/BP_Explosion.BP_Explosion_C" (Transformation|GetWorldTransform (Variables|Default|GetBomba)) "Undefined" 0 3e+01 0)
  (Actor|DestroyActor))

(event EventBeginPlay
  (bind _specialattack (Variables|Default|GetSpecialAttack))
  (Physics|AddForce (Variables|Default|GetBomba) (Math|Vector|MakeVector 0.0 0.0 (- 0.0 (Variables|Default|GetVelocidad%20caida))) "None" true)
  (Utilities|Struct|SetmembersinS_SpecialAttack _specialattack true)
  (Development|PrintString "Comienza cooldown")
  (Utilities|FlowControl|Delay 1.0)
  (Utilities|Struct|SetmembersinS_SpecialAttack _specialattack false)
  (Development|PrintString "Termina Cooldown"))

(fn ConstructionScript)