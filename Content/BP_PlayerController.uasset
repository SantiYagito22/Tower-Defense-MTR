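; Player controller that routes mouse and keyboard input to a support-drop system and to saving and loading.
; On BeginPlay it spawns a BP_SupportManager, which receives mouse movement to update the crosshair, right click to toggle it and left click to drop support.
; The K and L keys call the game mode's save and load functions (GuardarPartida, CargarPartida) on slot 0.
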(event EventBeginPlay
  (bind _returnvalue (Game|SpawnActorfromClass "/Game/Poderes/BP_SupportManager.BP_SupportManager_C" (Math|Conversions|ToTransform(Vector) "0, 0, 0") "Undefined" 0 0))
  (Variables|Default|SetSupportManager _returnvalue))

(event Input|MouseEvents|RightMouseButton
  (params (Key :type Key%20Structure :default "None"))
  (:Pressed
    (Default|ToggleCrosshair (Variables|Default|GetSupportManager) "NewEnumerator0")))

(event Input|MouseEvents|LeftMouseButton
  (params (Key :type Key%20Structure :default "None"))
  (:Pressed
    (Default|DropSupport (Variables|Default|GetSupportManager) "NewEnumerator0")))

(event Input|KeyboardEvents|L
  (params (Key :type Key%20Structure :default "None"))
  (:Pressed
    (bind _asmodo_juego (Utilities|Casting|CastToBP_GameMode (Game|GetGameMode)))
    (Default|CargarPartida _asmodo_juego)))

(event Input|KeyboardEvents|K
  (params (Key :type Key%20Structure :default "None"))
  (:Pressed
    (bind _asmodo_juego (Utilities|Casting|CastToBP_GameMode (Game|GetGameMode)))
    (Default|GuardarPartida _asmodo_juego)))

(event Input|MouseEvents|Mouse2D
  (params (AxisValue :type Vector :default "0, 0, 0"))
  (Default|UpdateCrosshairPositon (Variables|Default|GetSupportManager)))

(fn ConstructionScript)